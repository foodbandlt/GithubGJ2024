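; Game mode for a first-person house puzzle that plays background music and resolves interactions with named switches and doors.
; It reads and writes object states in a key-value map on FPPuzzleGameState, switching on object ID in InteractWithNamedObject.
; Light switches and the second bathroom door toggle, and certain states set key flags and refresh tagged key actors' visibility.
; Most other doors change state only once, while the front door always reports success.
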(event `self.ReceiveBeginPlay`
  (`GameplayStatics.PlaySound2D` "/Game/Sounds/BGMusic.BGMusic" 0.15 1.0 0.0 null null))

(fn `GetGameStateVariable`
  (params (Key :type String))
  (returns (Value :type Integer))
  (bind _asfppuzzle_game_state (cast `/Game/Player/Blueprints/FPPuzzleGameState` (`GameplayStatics.GetGameState`)))
  (return (`BlueprintMapLibrary.Map_Find` (`/Game/Player/Blueprints/FPPuzzleGameState.GameStateTracking` _asfppuzzle_game_state) Key)))

(fn `InteractWithNamedObject`
  (params (ObjectID :type String) (ObjectInteractedWith :type "Object Object Reference"))
  (returns (Success :type Boolean))
  (switch `string` ObjectID
    (:`LightSwitch1`
      (bind _value (`self.GetGameStateVariable` ObjectID :!label _label))
      (`/Engine/EditorBlueprintResources/StandardMacros.CompareInt` _value
        (:`>`
          (`self.SetGameStateVariable` ObjectID :!label _label_2))
        (:`==`
          (`self.SetGameStateVariable` ObjectID 1))
        (:`<`
          (goto _label_2)))
      (`|ExecutionSequence`
        (:`then_0`
          (switch `string` ObjectID
            (:`LightSwitch2`
              _)
            (:`LightSwitch6`
              _)
            (:`LightSwitch3`
              _))
          (bind _value_2 (`self.GetGameStateVariable` "LightSwitch2"))
          (bind _value_3 (`self.GetGameStateVariable` "LightSwitch6"))
          (bind _value_4 (`self.GetGameStateVariable` "LightSwitch3"))
          (if (and (== _value_2 0) (== _value_3 0) (== _value_4 0))
            (`self.SetGameStateVariable` "KitchenKey" 1)
            (else
              (`self.SetGameStateVariable` "KitchenKey")))
          (bind _outactors (`GameplayStatics.GetAllActorsWithTag` "KitchenKey"))
          (for _array_element _outactors
            (bind _asbp_kitchen_key (cast `/Game/Objects/Interactibles/InventoryItems/BP_KitchenKey` _array_element))
            (`/Game/Objects/Interactibles/InventoryItems/BP_KitchenKey.UpdateVisibility` _asbp_kitchen_key)))
        (:`then_1`
          (return true))))
    (:`LightSwitch2`
      (goto _label))
    (:`LightSwitch3`
      (goto _label))
    (:`LightSwitch4`
      (goto _label))
    (:`LightSwitch5`
      (goto _label))
    (:`LightSwitch6`
      (goto _label))
    (:`BedroomDoor1`
      (bind _value_5 (`self.GetGameStateVariable` ObjectID :!label _label_3))
      (`/Engine/EditorBlueprintResources/StandardMacros.CompareInt` _value_5
        (:`>`
          _)
        (:`==`
          (`self.SetGameStateVariable` ObjectID 1)
          (`|ExecutionSequence`
            (:`then_1`
              (return true))))
        (:`<`
          _))
      (return false))
    (:`BathroomDoor1`
      (goto _label_3))
    (:`BedroomDoor2`
      (goto _label_3))
    (:`BathroomDoor2`
      (bind _value_6 (`self.GetGameStateVariable` ObjectID))
      (`/Engine/EditorBlueprintResources/StandardMacros.CompareInt` _value_6
        (:`>`
          (`self.SetGameStateVariable` ObjectID :!label _label_4))
        (:`==`
          (`self.SetGameStateVariable` ObjectID 1))
        (:`<`
          (goto _label_4)))
      (bind _value_7 (`self.GetGameStateVariable` "BathroomDoor2"))
      (if (== _value_7 0)
        (`self.SetGameStateVariable` "BathroomKey" 1)
        (else
          (`self.SetGameStateVariable` "BathroomKey")))
      (bind _outactors_2 (`GameplayStatics.GetAllActorsWithTag` "BathroomKey"))
      (for _array_element_2 _outactors_2
        (bind _asbp_bathroom_key (cast `/Game/Objects/Interactibles/InventoryItems/BP_BathroomKey` _array_element_2))
        (`/Game/Objects/Interactibles/InventoryItems/BP_BathroomKey.UpdateVisibility` _asbp_bathroom_key)
        (return true)))
    (:`LaundryDoor`
      (goto _label_3))
    (:`GarageDoor`
      (goto _label_3))
    (:`FrontDoor`
      (return true))))

(fn `SetGameStateVariable`
  (params (Key :type String) (Value :type Integer))
  (bind _asfppuzzle_game_state (cast `/Game/Player/Blueprints/FPPuzzleGameState` (`GameplayStatics.GetGameState`)))
  (bind _gamestatetracking (`/Game/Player/Blueprints/FPPuzzleGameState.GameStateTracking` _asfppuzzle_game_state))
  (`BlueprintMapLibrary.Map_Add` _gamestatetracking Key Value)
  (set `/Game/Player/Blueprints/FPPuzzleGameState.GameStateTracking` _gamestatetracking _asfppuzzle_game_state))

(fn `UserConstructionScript`)
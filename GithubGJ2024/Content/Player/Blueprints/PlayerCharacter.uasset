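; Player character that handles camera-relative movement, look input and selection of interactable actors in view.
; BeginPlay adds the Enhanced Input mapping and starts a looping timer that line traces a short distance from the camera for WorldDynamic objects.
; Hit actors implementing the SelectActors interface are selected through interface messages, and the previous one is deselected when the target changes or is lost.
; The interact input currently only prints the selected actor's name.
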(event `self.ReceiveBeginPlay`
  (bind _returnvalue (pcsubsystem `EnhancedInputLocalPlayerSubsystem` (`GameplayStatics.GetPlayerController` 0)))
  ;[1 1 1] On Play
  (`/Engine/EditorBlueprintResources/StandardMacros.IsValid` _returnvalue
    (:`Is Valid`
      (`EnhancedInputSubsystemInterface.AddMappingContext` _returnvalue "/Game/Player/Input/P_InputMapping.P_InputMapping" 0 (struct))
      (`KismetSystemLibrary.K2_SetTimerDelegate` (delegate `CheckSightLine`) 0.2 true))))

(event `CheckSightLine`
  ;[1 1 1] On Play
  (`self.LineTraceForInteractables`))

(event `EnhancedInput|/Game/Player/Input/InputActions/IA_Movement`
  (params (ActionValue :type "Vector2D Structure") (ElapsedSeconds :type "Float (double-precision)") (TriggeredSeconds :type "Float (double-precision)") (InputAction :type "InputAction Object Reference" :default "/Game/Player/Input/InputActions/IA_Movement.IA_Movement"))
  ;[1 1 1] Movement/Camera
  (:`Triggered`
    (`self.AddMovementInput` (`self.Movement` ActionValue))))

(event `EnhancedInput|/Game/Player/Input/InputActions/IA_Camera`
  (params (ActionValue :type "Vector2D Structure") (ElapsedSeconds :type "Float (double-precision)") (TriggeredSeconds :type "Float (double-precision)") (InputAction :type "InputAction Object Reference" :default "/Game/Player/Input/InputActions/IA_Camera.IA_Camera"))
  (bind (_x _y) (`KismetMathLibrary.BreakVector2D` ActionValue))
  ;[1 1 1] Movement/Camera
  (:`Triggered`
    (`self.AddControllerYawInput` (* (`self.Horizontal Look Sensitivity`) _x))
    (`self.AddControllerPitchInput` (* (`self.Vertical Look Sensitivity`) _y))))

(event `EnhancedInput|/Game/Player/Input/InputActions/IA_Interact`
  (params (ActionValue :type Boolean) (ElapsedSeconds :type "Float (double-precision)") (TriggeredSeconds :type "Float (double-precision)") (InputAction :type "InputAction Object Reference" :default "/Game/Player/Input/InputActions/IA_Interact.IA_Interact"))
  (bind _selectedactor (`self.SelectedActor`))
  ;[1 1 1] Interact
  (:`Triggered`
    (`/Engine/EditorBlueprintResources/StandardMacros.IsValid` _selectedactor
      (:`Is Valid`
        (`KismetSystemLibrary.PrintString` (`KismetSystemLibrary.GetDisplayName` _selectedactor))))))

(fn `LineTraceForInteractables`
  (bind _returnvalue (`GameplayStatics.GetPlayerCameraManager` 0))
  (bind _selectedactor (`self.SelectedActor`))
  (bind _selectedactor_2 (`self.SelectedActor`))
  (bind _returnvalue_2 (`PlayerCameraManager.GetCameraLocation` _returnvalue))
  (bind (_outhit _returnvalue_3) (`KismetSystemLibrary.LineTraceSingleForObjects` _returnvalue_2 (+ _returnvalue_2 (* (`SceneComponent.GetForwardVector` (`PlayerCameraManager.TransformComponent` _returnvalue)) (175.0 175.0 175.0))) (`|MakeArray` "ObjectTypeQuery2" :!type "EObjectTypeQuery Enum")))
  (if _returnvalue_3
    (if (`KismetSystemLibrary.DoesImplementInterface` (`.HitActor` (`GameplayStatics.BreakHitResult` _outhit)) "/Game/Objects/Interactibles/SelectActors.SelectActors_C")
      (bind _isselected_ (message `/Game/Objects/Interactibles/SelectActors.isSelected?` (`.HitActor` (`GameplayStatics.BreakHitResult` _outhit))))
      (if (not _isselected_)
        (`/Engine/EditorBlueprintResources/StandardMacros.IsValid` _selectedactor
          (:`Is Valid`
            (message `/Game/Objects/Interactibles/SelectActors.DeselectMyActor` _selectedactor)
            (set `self.SelectedActor` null))
          (:`Is Not Valid`
            _))
        (message `/Game/Objects/Interactibles/SelectActors.SelectMyActor` (`.HitActor` (`GameplayStatics.BreakHitResult` _outhit)))
        (set `self.SelectedActor` (`.HitActor` (`GameplayStatics.BreakHitResult` _outhit))))
      (else
        (`/Engine/EditorBlueprintResources/StandardMacros.IsValid` _selectedactor_2 :!label _label
          (:`Is Valid`
            (message `/Game/Objects/Interactibles/SelectActors.DeselectMyActor` _selectedactor_2)
            (set `self.SelectedActor` null)))))
    (else
      (goto _label))))

(fn `Movement`
  (params (InVec :type "Vector2D Structure"))
  (returns (ReturnValue :type "Vector Structure"))
  (bind (_x _y) (`KismetMathLibrary.BreakVector2D` InVec))
  (bind _camera (`self.Camera`))
  (return (+ (* (`SceneComponent.GetForwardVector` _camera) _y) (* (`SceneComponent.GetRightVector` _camera) _x))))

(fn `UserConstructionScript`)